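; BP_Egg is a chicken egg actor that, when fertile, hatches into an actor of its mother's class after a delay.
; Hatching destroys the egg and only happens while the BP_Chicken count is below the mother's population limit; otherwise the egg becomes infertile.
; BeginPlay also plays a feather particle burst and enables Tick from the player character's Debug flag, which draws the fertility state as debug text.
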(event `self.ReceiveBeginPlay`
  ;[0 0 0] Spawn chicken from egg
  (`|ExecutionSequence`
    (:`then_0`
      (if (`self.Fertile?`)
        (`KismetSystemLibrary.Delay` (`self.Delay to hatch`))
        (bind _outactors (`GameplayStatics.GetAllActorsOfClass` "/Game/ChickenAI/Blueprints/Chicken/Chicken/BP_Chicken.BP_Chicken_C"))
        (if (< (`KismetArrayLibrary.Array_Length` _outactors) (`/Game/ChickenAI/Blueprints/Chicken/Chicken/BP_Chicken.Max level population ` (`self.Mother`)))
          (`|SpawnActorFromClass` (`self.Mother class`) (`KismetMathLibrary.MakeTransform` (`SceneComponent.K2_GetComponentLocation` (`self.Egg`))) "AdjustIfPossibleButAlwaysSpawn" "SelectDefaultAtRuntime" null null)
          (`self.K2_DestroyActor`)
          (else
            (set `self.Fertile?` false)))))
    (:`then_1`
      ;[1 0 0.7796] Start debug
      (bind _asfirst_person_character (cast `/Game/ChickenAI/Demo/UnrealContent/FirstPersonBP/Blueprints/FirstPersonCharacter` (`GameplayStatics.GetPlayerPawn` 0)))
      (`self.SetActorTickEnabled` (`/Game/ChickenAI/Demo/UnrealContent/FirstPersonBP/Blueprints/FirstPersonCharacter.Debug` _asfirst_person_character)))
    (:`then_2`
      ;[1 0.1019 0.8813] Cosmetic particles when spawning egg
      (`GameplayStatics.SpawnEmitterAttached` "/Game/ChickenAI/Demo/Particles/P_FeatherExplosion.P_FeatherExplosion" (`self.Egg`)))))

(event `self.ReceiveTick`
  (params (DeltaSeconds :type "Float (single-precision)"))
  ;[1 0 0.5896] Draw debug text
  (`KismetSystemLibrary.DrawDebugString` (`self.K2_GetActorLocation`) (`KismetMathLibrary.SelectString` "Fertilized egg" "Unfertilized egg" (`self.Fertile?`)) null))

(fn `UserConstructionScript`)