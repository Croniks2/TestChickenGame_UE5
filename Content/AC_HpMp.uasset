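; AC_HpMp is a component that holds a character's current and maximum HP and MP.
; Setter functions write the maximums together and each current value separately, with no clamping.
; GetStatsForHUD returns all four values as truncated integer text, plus HP and MP progress bar fractions normalized against their maximums.
; The event graph does nothing.
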(event `self.ReceiveBeginPlay`)

(fn `Get Stats for HUD`
  (returns (MaxHP :type Text) (CurrentHP :type Text) (HPProgressBar :type "Float (double-precision)") (MaxMP :type Text) (CurrentMP :type Text) (MPProgressBar :type "Float (double-precision)"))
  (bind _currenthp (`self.CurrentHP`))
  (bind _maxmp (`self.MaxMP`))
  (bind _currentmp (`self.CurrentMP`))
  (bind _maxhp (`self.MaxHP`))
  (return (`KismetTextLibrary.Conv_IntToText` (`KismetMathLibrary.FTrunc` _maxhp)) (`KismetTextLibrary.Conv_IntToText` (`KismetMathLibrary.FTrunc` _currenthp)) (`KismetMathLibrary.NormalizeToRange` _currenthp 0.0 _maxhp) (`KismetTextLibrary.Conv_IntToText` (`KismetMathLibrary.FTrunc` _maxmp)) (`KismetTextLibrary.Conv_IntToText` (`KismetMathLibrary.FTrunc` _currentmp)) (`KismetMathLibrary.NormalizeToRange` _currentmp 0.0 _maxmp)))

(fn `SetCurrentHP`
  (params (CurrentHP :type "Float (double-precision)"))
  (set `self.CurrentHP` CurrentHP))

(fn `SetCurrentMP`
  (params (CurrentMP :type "Float (double-precision)"))
  (set `self.CurrentMP` CurrentMP))

(fn `SetMaxHPAndMaxMP`
  (params (MaxHP :type "Float (double-precision)") (MaxMP :type "Float (double-precision)"))
  (set `self.MaxHP` MaxHP)
  (set `self.MaxMP` MaxMP))