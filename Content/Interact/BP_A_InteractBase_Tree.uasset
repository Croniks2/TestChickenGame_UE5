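; Interactable tree actor that yields wood when harvested and falls over once depleted.
; Interact checks IsInteract, which allows use while the wood charge count is below its maximum, then increments the count and returns a small random amount of Wood.
; When the last charge is used, the static mesh starts simulating physics and receives a fixed velocity-change impulse to topple it.
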(fn `Interact`
  (returns (ResourceName :type Name) (ResourceAmount :type Integer))
  (bind _staticmesh (`self.StaticMesh`))
  (bind _caninteract (`self.IsInteract`))
  (if _caninteract
    (bind _result (`/Engine/EditorBlueprintResources/StandardMacros.IncrementInt` (`self.currentWoodCharges`))
      (:`  `
        (set `self.currentWoodCharges` _result)
        (bind _caninteract_2 (`self.IsInteract`))
        (if (not _caninteract_2)
          (`PrimitiveComponent.SetSimulatePhysics` _staticmesh true)
          (`PrimitiveComponent.AddImpulse` _staticmesh (190.0 190.0 50.0) "None" true))
        (return "Wood" (`KismetMathLibrary.RandomIntegerInRange` 1 5))))))

(fn `IsInteract`
  (returns (canInteract :type Boolean))
  (`/Engine/EditorBlueprintResources/StandardMacros.CompareInt` (`self.currentWoodCharges`) (`self.maxWoodCharges`)
    (:`>`
      _)
    (:`==`
      _)
    (:`<`
      (return true)))
  (return false))

(fn `UserConstructionScript`
  (`parent.UserConstructionScript`))