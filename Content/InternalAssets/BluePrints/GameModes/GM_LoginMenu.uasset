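; Game mode for the login menu that loads the local user accounts save data.
; On BeginPlay with authority, it creates and saves an empty SG_Users object to the "Accounts" slot if none exists, then loads that slot.
; The loaded save is cached as SGUsers and exposed through a getter function for other Blueprints.
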(event `self.ReceiveBeginPlay`
  (`/Engine/EditorBlueprintResources/ActorMacros.Switch Has Authority`
    (:`Authority`
      (bind _returnvalue (`GameplayStatics.DoesSaveGameExist` "Accounts"))
      (if (not _returnvalue)
        (bind _returnvalue_2 (`GameplayStatics.CreateSaveGameObject` "/Game/InternalAssets/SaveGame/SG_Users.SG_Users_C"))
        (`GameplayStatics.SaveGameToSlot` _returnvalue_2 "Accounts"))
      (bind _returnvalue_3 (`GameplayStatics.LoadGameFromSlot` "Accounts"))
      (bind _assg_users (cast `/Game/InternalAssets/SaveGame/SG_Users` _returnvalue_3))
      (set `self.SG_Users` _assg_users))))

(fn `Get_SG_Users`
  (returns (SG_Users :type "/Game/InternalAssets/SaveGame/SG_Users Object Reference"))
  (return (`self.SG_Users`)))

(fn `UserConstructionScript`
  (`parent.UserConstructionScript`))