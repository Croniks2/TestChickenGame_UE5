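; Player controller for the login menu that sets the view to a camera actor, shows the cursor and handles login attempts.
; Server-named events read users from the game mode's SG_Users via an interface, compare plain-text credentials, then open NonThirdPersonMape or print errors through a client-named event.
; The "User not found" branch is unreachable because its in-loop index check never fails.
; Registration is unfinished, only fetching the user list.
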(event `self.ReceiveBeginPlay`
  ;[1 1 1] LoginLogic
  (set `self.bShowMouseCursor` true)
  (bind _outactors (`GameplayStatics.GetAllActorsOfClass` "/Script/Engine.CameraActor"))
  (bind _output_get (set `self.MainCamera` (`|GetArrayItem` _outactors)))
  (`self.SetViewTargetWithBlend` _output_get))

(event `/Game/InternalAssets/BluePrints/PlayerControllers/LoginMenu/BPI/BPI_PC_LoginMenu.TryToEnterGame`
  (params (UserName :type String) (UserPassword :type String))
  ;[1 1 1] LoginLogic
  (`self.EnterGameOnServer_Event` UserName UserPassword))

(event `EnterGameOnServer_Event`
  (params (Login :type String) (Password :type String))
  ;[1 1 1] LoginLogic
  (bind _asbpi_gm_login_menu (cast `/Game/InternalAssets/BluePrints/GameModes/BPI_GM_LoginMenu` (`GameplayStatics.GetGameMode`)))
  (bind _sg_users (`/Game/InternalAssets/BluePrints/GameModes/BPI_GM_LoginMenu.Get_SG_Users` _asbpi_gm_login_menu))
  (bind _userinfos (`/Game/InternalAssets/SaveGame/BPI/BPI_SG_Users.GetUsers` _sg_users))
  (bind _returnvalue (`KismetArrayLibrary.Array_Length` _userinfos))
  (if (> _returnvalue 0)
    (for (_array_element _array_index) _userinfos
      (bind (_username _userpassword) (break `/Game/InternalAssets/SaveGame/Structs/S_Users` _array_element))
      (if (`KismetStringLibrary.NotEqual_StrStr` _username Login)
        (if (not (< _array_index _returnvalue))
          (`self.EnterGameErrorOnClient_Event` "User not found"))
        (elif (`KismetStringLibrary.NotEqual_StrStr` _userpassword Password)
          (`self.EnterGameErrorOnClient_Event` "Incorrect password")
          (break)
          (else
            (`GameplayStatics.OpenLevel` "NonThirdPersonMape")))))
    (else
      (`self.EnterGameErrorOnClient_Event` "No users in SG_Users"))))

(event `EnterGameErrorOnClient_Event`
  (params (Message :type Text))
  ;[1 1 1] LoginLogic
  (`KismetSystemLibrary.PrintText` Message))

(event `/Game/InternalAssets/BluePrints/PlayerControllers/LoginMenu/BPI/BPI_PC_LoginMenu.TryToRegister`
  (params (UserName :type String) (UserPassword :type String) (RepeatUserPassword :type String))
  (`self.RegisterGameOnServer_Event` UserName UserPassword RepeatUserPassword))

(event `RegisterGameOnServer_Event`
  (params (Login :type String) (Password :type String) (Password2 :type String))
  (bind _asbpi_gm_login_menu (cast `/Game/InternalAssets/BluePrints/GameModes/BPI_GM_LoginMenu` (`GameplayStatics.GetGameMode`)))
  (bind _sg_users (`/Game/InternalAssets/BluePrints/GameModes/BPI_GM_LoginMenu.Get_SG_Users` _asbpi_gm_login_menu))
  (`/Game/InternalAssets/SaveGame/BPI/BPI_SG_Users.GetUsers` _sg_users))

(fn `UserConstructionScript`
  (`parent.UserConstructionScript`))